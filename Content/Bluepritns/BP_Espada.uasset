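; BP_Espada is a sword pickup that the Player collects by overlapping it.
; On overlap it halts the player's movement and sets the TengoEsp and AgarreItemAnim flags for the pickup animation.
; After a short delay it hides itself, restores walking, sets its own TieneEspada flag and destroys itself.
; A sprite color-flash event, AgarraItem, exists, but its timer setup is disconnected and never runs.
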(event Custom|AgarraItem
  (bind _as_player (Variables|Default|GetAs%20Player))
  (bind _sprite (Variables|/Script/Paper2D.PaperCharacter|GetSprite _as_player))
  (Utilities|FlowControl|FlipFlop
    (:A
      (Sprite|SetSpriteColor _sprite "(R=0.588542,G=0.248804,B=0.007067,A=1.000000)")
      (Utilities|FlowControl|Delay 0.1))
    (:B
      (Sprite|SetSpriteColor _sprite "(R=1.000000,G=1.000000,B=1.000000,A=1.000000)"))))

(event EventBeginPlay)

(event Collision|EventActorBeginOverlap
  (params (OtherActor :type Actor%20Object%20Reference))
  (bind _asplayer (Utilities|Casting|CastToPlayer OtherActor))
  (bind _output_get (Variables|Default|SetAs%20Player _asplayer))
  (Pawn|Components|CharacterMovement|SetMovementMode (Variables|/Script/Engine.Character|GetCharacterMovement _output_get) "MOVE_None" 0)
  (Components|Movement|StopMovementImmediately (Variables|/Script/Engine.Character|GetCharacterMovement _output_get))
  (Variables|/Game/Personaje/Player.Player_C|SetTengoEsp? _output_get true)
  (Variables|/Game/Personaje/Player.Player_C|SetAgarreItemAnim _output_get true)
  (Utilities|FlowControl|Delay 1.0)
  (Rendering|SetActorHiddenInGame true)
  (Variables|/Game/Personaje/Player.Player_C|SetAgarreItemAnim (Variables|Default|GetAs%20Player) false)
  (Pawn|Components|CharacterMovement|SetMovementMode (Variables|/Script/Engine.Character|GetCharacterMovement (Variables|Default|GetAs%20Player)) "MOVE_Walking" 0)
  (Variables|Default|SetTiene%20Espada true)
  (Utilities|FlowControl|Delay 0.2)
  (Actor|DestroyActor))

(event EventTick
  (params (DeltaSeconds :type Float%20%28single-precision%29)))

(fn ConstructionScript)