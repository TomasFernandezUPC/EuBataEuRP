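; BP_ITEMVIDA is a pickup that adds a healing orb (OrbeCuracion) to the count when the player overlaps its sphere.
; On BeginPlay it caches the GM_HUD game instance, where the orb count is stored.
; The overlap increments that count up to a fixed cap, prints it, refreshes the player's HudVida widget through UpdateOrbe, then destroys the pickup.
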(event OnComponentBeginOverlap(Sphere)
  (params (OverlappedComponent :type Primitive%20Component%20Object%20Reference) (OtherActor :type Actor%20Object%20Reference) (OtherComp :type Primitive%20Component%20Object%20Reference) (OtherBodyIndex :type Integer) (bFromSweep :type Boolean) (SweepResult :type Hit%20Result%20Structure%20%28by%20ref%29))
  (bind _as_gm_hud (Variables|Default|GetAs%20GM%20HUD))
  (bind _asplayer (Utilities|Casting|CastToPlayer OtherActor))
  (if (>= (+ (Variables|/Game/Bluepritns/GM_HUD.GM_HUD_C|GetOrbeCuracion _as_gm_hud) 1.0) 1e+01)
    (Variables|/Game/Bluepritns/GM_HUD.GM_HUD_C|SetOrbeCuracion (Variables|Default|GetAs%20GM%20HUD) 1e+01)
    (else
      (bind _output_get (Variables|/Game/Bluepritns/GM_HUD.GM_HUD_C|SetOrbeCuracion _as_gm_hud (+ (Variables|/Game/Bluepritns/GM_HUD.GM_HUD_C|GetOrbeCuracion _as_gm_hud) 1.0)))))
  (Development|PrintString (Utilities|String|ToString(Float) _output_get))
  (Default|UpdateOrbe (Variables|/Game/Personaje/Player.Player_C|GetHudVida _asplayer) (Variables|/Game/Bluepritns/GM_HUD.GM_HUD_C|GetOrbeCuracion (Variables|Default|GetAs%20GM%20HUD)) 1e+01)
  (Actor|DestroyActor))

(event EventBeginPlay
  (bind _asgm_hud (Utilities|Casting|CastToGM_HUD (Game|GetGameInstance)))
  (Variables|Default|SetAs%20GM%20HUD _asgm_hud))

(event EventTick
  (params (DeltaSeconds :type Float%20%28single-precision%29)))

(fn ConstructionScript)