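; Aflicción is a PaperZD ranged enemy that shoots projectiles at pawns it sees and drops an item on death.
; PawnSensing sightings trigger a delayed attack animation, whose end spawns Aflicción_proyectil aimed at the pawn.
; Damage lowers Life and plays a hurt animation; at zero, Memori blocks further hits, collision and movement stop, and the death animation leads to a BP_RANGEITEM drop and self-destruction.
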(event OnSeePawn(PawnSensing)
  (params (Pawn :type Pawn%20Object%20Reference))
  (bind _returnvalue (Transformation|GetActorTransform))
  (if (not (Variables|Default|Getmemori?))
    (Utilities|FlowControl|Delay 1.3)
    (if (not (Variables|Default|Getmemori?))
      (|PlayAnimationOverridewithCallbacks (Variables|/Script/PaperZD.PaperZDAnimationComponent|GetAnimInstance (Variables|Default|GetPaperZDAnimation)) "/Game/Enemigo/AnimSequences/AFATKS.AFATKS" "DefaultSlot" 1.0 0.0
        (:then
          (Variables|Default|SetAtaqueRango true))
        (:OnCompleted
          (Variables|Default|SetAtaqueRango false :!label _label)
          (Game|SpawnActorfromClass "/Game/Bluepritns/Balas/Aflicción_proyectil.Aflicción_proyectil_C" (Math|Transform|MakeTransform (Math|Vector|MakeVector (.x (.location _returnvalue)) (.y (.location _returnvalue)) (- (.z (.location _returnvalue)) 5e+01)) (.rotation _returnvalue) (.scale _returnvalue)) "Undefined" "MultiplyWithRoot" 0 (* (Math|Vector|Normalize (- (Transformation|GetActorLocation Pawn) (Transformation|GetActorLocation))) 5.5e+02) 0))
        (:OnCancelled
          (goto _label))))))

(event EventBeginPlay)

(event Collision|EventActorBeginOverlap
  (params (OtherActor :type Actor%20Object%20Reference))
  (|CallParentFunction OtherActor) ; Este nodo está deshabilitado y no se le llamará.\nArrastra pines para construir una funcionalidad.
)

(event EventTick
  (params (DeltaSeconds :type Float%20%28single-precision%29))
  (|CallParentFunction DeltaSeconds) ; Este nodo está deshabilitado y no se le llamará.\nArrastra pines para construir una funcionalidad.
)

(event Game|Damage|EventAnyDamage
  (params (Damage :type Float%20%28single-precision%29) (DamageType :type Damage%20Type%20Object%20Reference) (InstigatedBy :type Controller%20Object%20Reference) (DamageCauser :type Actor%20Object%20Reference))
  (bind _self self)
  (bind _charactermovement (Variables|Character|GetCharacterMovement))
  (bind _returnvalue (Transformation|GetActorTransform _self))
  (if (not (Variables|Default|Getmemori?))
    (bind _output_get (Variables|Default|SetLife (- (Variables|Default|GetLife) Damage)))
    (if (<= _output_get 0.0)
      (Variables|Default|Setmemori? true)
      (Collision|SetCollisionEnabled (Variables|Default|GetCapsuleComponent) "NoCollision")
      (Pawn|Components|CharacterMovement|SetMovementMode _charactermovement "MOVE_None" 0)
      (Components|Movement|StopMovementImmediately _charactermovement)
      (|PlayAnimationOverridewithCallbacks (Variables|/Script/PaperZD.PaperZDAnimationComponent|GetAnimInstance (Variables|Default|GetPaperZDAnimation)) "/Game/Enemigo/AnimSequences/AFDEATH.AFDEATH" "DefaultSlot" 1.0 0.0
        (:OnCompleted
          _)
        (:OnCancelled
          _))
      (Utilities|FlowControl|Delay 2.0)
      (Game|SpawnActorfromClass "/Game/Bluepritns/BP_RANGEITEM.BP_RANGEITEM_C" (Math|Transform|MakeTransform (Math|Vector|MakeVector (.x (.location _returnvalue)) (.y (.location _returnvalue)) (- (.z (.location _returnvalue)) 1.5e+02)) (.rotation _returnvalue) (.scale _returnvalue)) "Undefined" "MultiplyWithRoot" 0 0)
      (Actor|DestroyActor)
      (else
        (|PlayAnimationOverridewithCallbacks (Variables|/Script/PaperZD.PaperZDAnimationComponent|GetAnimInstance (Variables|Default|GetPaperZDAnimation)) "/Game/Enemigo/AnimSequences/AFHURT.AFHURT" "DefaultSlot" 1.0 0.0
          (:then
            (Variables|Default|Sethurt true)
            (Utilities|FlowControl|Delay 0.2))
          (:OnCompleted
            (Variables|Default|Sethurt false :!label _label))
          (:OnCancelled
            (goto _label)))))))

(fn ConstructionScript
  (|CallParentFunction))