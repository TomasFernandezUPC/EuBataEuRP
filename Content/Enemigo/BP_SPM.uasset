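; BP_SPM is a PaperZD-animated enemy that chases seen pawns, attacks and can die.
; On sight it moves to the pawn and, after a short delay, attacks, damaging "PY"-tagged actors in its Box.
; Sighting also starts a looping timer that moves it to random nearby reachable points.
; Damage plays hurt or death animations; Memori marks death, which calls CallEnemyOnDie and randomly spawns BP_ITEMVIDA before destroying the actor.
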(event OnSeePawn(PawnSensing)
  (params (Pawn :type Pawn%20Object%20Reference))
  (Utilities|FlowControl|Sequence
    (:then_0
      (AI|AIMoveTo self "0, 0, 0" Pawn 3.0 false
        (:OnSuccess
          (Utilities|FlowControl|Delay 1.0)
          (if (not (Variables|Default|Getmemori?))
            (|PlayAnimationOverridewithCallbacks (Variables|/Script/PaperZD.PaperZDAnimationComponent|GetAnimInstance (Variables|Default|GetPaperZDAnimation)) "/Game/Enemigo/AnimSequences/SMSQ_ATTACK.SMSQ_ATTACK" "DefaultSlot" 1.0 0.0
              (:then
                (Variables|Default|SetTeataco? true)
                (CallFunction|Hitcheck))
              (:OnCompleted
                (Variables|Default|SetTeataco? false :!label _label))
              (:OnCancelled
                (goto _label)))))))
    (:then_1
      (Utilities|Time|SetTimerbyEvent (delegate Custom|CustomEvent) 2.0 true))))

(event Custom|CustomEvent
  (if (not (Variables|Default|Getmemori?))
    (AI|AIMoveTo self (.RandomLocation (AI|Navigation|GetRandomReachablePointinRadius (Transformation|GetActorLocation) 5e+02 0 0)) 0 5.0 false
      (:then
        (Variables|Default|Setmuevo true :!label _label))
      (:OnSuccess
        (goto _label))
      (:OnFail
        (Variables|Default|Setmuevo false)))))

(event EventBeginPlay)

(event Collision|EventActorBeginOverlap
  (params (OtherActor :type Actor%20Object%20Reference))
  (|CallParentFunction OtherActor) ; Este nodo está deshabilitado y no se le llamará.\nArrastra pines para construir una funcionalidad.
)

(event EventTick
  (params (DeltaSeconds :type Float%20%28single-precision%29))
  (|CallParentFunction DeltaSeconds) ; Este nodo está deshabilitado y no se le llamará.\nArrastra pines para construir una funcionalidad.
)

(event Game|Damage|EventAnyDamage
  (params (Damage :type Float%20%28single-precision%29) (DamageType :type Damage%20Type%20Object%20Reference) (InstigatedBy :type Controller%20Object%20Reference) (DamageCauser :type Actor%20Object%20Reference))
  (bind _charactermovement (Variables|Character|GetCharacterMovement))
  (if (not (Variables|Default|Getmemori?))
    (bind _output_get (Variables|Default|SetLife (- (Variables|Default|GetLife) Damage)))
    (if (<= _output_get 0.0)
      (Collision|SetCollisionEnabled (Variables|Default|GetCapsuleComponent) "NoCollision")
      (Pawn|Components|CharacterMovement|SetMovementMode _charactermovement "MOVE_None" 0)
      (Components|Movement|StopMovementImmediately _charactermovement)
      (Variables|Default|Setmemori? true)
      (|PlayAnimationOverridewithCallbacks (Variables|/Script/PaperZD.PaperZDAnimationComponent|GetAnimInstance (Variables|Default|GetPaperZDAnimation)) "/Game/Enemigo/AnimSequences/SMSQ_DEATH.SMSQ_DEATH" "DefaultSlot" 1.0 0.0
        (:OnCompleted
          _)
        (:OnCancelled
          _))
      (Utilities|FlowControl|Delay 2.0)
      (Default|CallEnemyonDie self)
      (if (Math|Random|RandomBool)
        (Actor|DestroyActor)
        (else
          (Game|SpawnActorfromClass "/Game/Bluepritns/BP_ITEMVIDA.BP_ITEMVIDA_C" (Transformation|GetActorTransform) "Undefined" "MultiplyWithRoot" 0 0)
          (Actor|DestroyActor)))
      (else
        (|PlayAnimationOverridewithCallbacks (Variables|/Script/PaperZD.PaperZDAnimationComponent|GetAnimInstance (Variables|Default|GetPaperZDAnimation)) "/Game/Enemigo/AnimSequences/SMSQ_HURT.SMSQ_HURT" "DefaultSlot" 1.0 0.0
          (:then
            (Variables|Default|Sethurt true))
          (:OnCompleted
            (Variables|Default|Sethurt false :!label _label))
          (:OnCancelled
            (goto _label)))))))

(fn ConstructionScript
  (|CallParentFunction))

(fn Hitcheck
  (for _array_element (Collision|GetOverlappingActors (Variables|Default|GetBox) "/Game/Personaje/Player.Player_C" :!class /Script/Engine.PrimitiveComponent)
    (if (!= _array_element self)
      (if (Actor|ActorHasTag _array_element "PY")
        (Game|Damage|ApplyDamage _array_element 7.0 0 0)))))